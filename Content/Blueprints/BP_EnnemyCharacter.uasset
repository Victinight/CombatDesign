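; Enemy character Blueprint that handles health, damage and hit reactions.
; On BeginPlay it hands the health bar from its widget to BPCStats and, for one character type, sets health from an enemy health value.
; AnyDamage is gated by a getting-hit flag, which this graph never clears; after a short retriggerable delay it subtracts damage through BPCStats and calls HitReact.
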(event EventBeginPlay
  (bind _aswb_ennemy_health (Utilities|Casting|CastToWB_EnnemyHealth (UserInterface|GetWidget (Variables|Default|GetWidget))))
  (Default|SetHealthBarProgress (Variables|Default|GetBPC_Stats) (Variables|/Game/UI/WB_EnnemyHealth.WB_EnnemyHealth_C|GetHealthBar _aswb_ennemy_health))
  (if (Utilities|Enum|Equal(Enum) (Variables|Default|GetEnum_CharacterType) "NewEnumerator1")
    (Variables|Default|SetFloat_Health (Variables|Default|GetEnnemyHeatlh))))

(event Game|Damage|EventAnyDamage
  (params (Damage :type Float%20%28single-precision%29) (DamageType :type Damage%20Type%20Object%20Reference) (InstigatedBy :type Controller%20Object%20Reference) (DamageCauser :type Actor%20Object%20Reference))
  (if (not (Variables|Default|GetBool_GettingHit))
    (Variables|Default|SetBool_GettingHit true)
    (Utilities|FlowControl|RetriggerableDelay 0.15)
    (Default|IncreaseValue (Variables|Default|GetBPC_Stats) "NewEnumerator1" (* Damage -1.0))
    (CallFunction|HitReact)))

(fn ConstructionScript
  (|CallParentFunction))