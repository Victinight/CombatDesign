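; BP_WeaponPickable is a weapon pickup actor that equips its weapon on a character that walks into it.
; The construction script sets its static mesh from WeaponData.
; On PickUpTrigger overlap, it casts to BP_ThirdPersonCharacter, checks for one specific character type, passes WeaponData to EquipWeapon and destroys itself.
; An unconnected alternative using BPI_Interact is present but never runs.
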(event OnComponentBeginOverlap(PickUpTrigger)
  (params (OverlappedComponent :type Primitive%20Component%20Object%20Reference) (OtherActor :type Actor%20Object%20Reference) (OtherComp :type Primitive%20Component%20Object%20Reference) (OtherBodyIndex :type Integer) (bFromSweep :type Boolean) (SweepResult :type Hit%20Result%20Structure%20%28by%20ref%29))
  (bind _asbp_third_person_character (Utilities|Casting|CastToBP_ThirdPersonCharacter OtherActor))
  (if (Utilities|Enum|Equal(Enum) (Variables|/Game/ThirdPerson/Blueprints/BP_ThirdPersonCharacter.BP_ThirdPersonCharacter_C|GetEnum_CharacterType _asbp_third_person_character) "NewEnumerator0")
    (Default|EquipWeapon _asbp_third_person_character (Variables|Default|GetWeaponData))
    (Actor|DestroyActor)))

(event EventBeginPlay)

(event Collision|EventActorBeginOverlap
  (params (OtherActor :type Actor%20Object%20Reference)))

(event EventTick
  (params (DeltaSeconds :type Float%20%28single-precision%29)))

(fn ConstructionScript
  (Components|StaticMesh|SetStaticMesh (Variables|Default|GetStaticMesh) (Variables|/Game/Blueprints/Weapons/BP_DA_Wepon.BP_DA_Wepon_C|GetStaticmesh (Variables|Default|GetWeaponData))))