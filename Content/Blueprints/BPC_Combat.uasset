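; Player combat component for BP_ThirdPersonCharacter that handles target lock and a stamina-gated dodge roll.
; Lock toggles via a camera-forward sphere trace for pawns, attaches a marker actor, switches movement to controller-facing, and Tick aims control rotation at the target.
; Roll plays a directional montage chosen from the stored ZQSD key when locked, otherwise forward.
; Delays after montage start time the dodge flags, rotation rate, stamina cost and regen pause.
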(event Custom|DestroyWidget
  (params (DestroyedActor :type Actor%20Object%20Reference))
  ;[0.2708 0.2708 0.2708 0.5] Target Lock
  (Actor|DestroyActor (Variables|Default|GetTargetLockWidget)))

(event Input|EnhancedActionEvents|EnhancedInputActionIA_Roll
  (params (ActionValue :type Boolean) (ElapsedSeconds :type Float%20%28double-precision%29) (TriggeredSeconds :type Float%20%28double-precision%29) (InputAction :type Input%20Action%20Object%20Reference :default "/Game/Input/Actions/IA_Roll.IA_Roll"))
  (bind _ref_playerbp (Variables|Default|GetRef_PlayerBP))
  (bind _bpc_stats (Variables|/Game/ThirdPerson/Blueprints/BP_ThirdPersonCharacter.BP_ThirdPersonCharacter_C|GetBPC_Stats _ref_playerbp))
  ;[0.2708 0.2708 0.2708 0.5] Roll
  (:Started
    (if (>= (Variables|/Game/Blueprints/BPC_Stats.BPC_Stats_C|GetStamina (Variables|/Game/ThirdPerson/Blueprints/BP_ThirdPersonCharacter.BP_ThirdPersonCharacter_C|GetBPC_Stats (Variables|Default|GetRef_PlayerBP))) 15.0)
      (Utilities|FlowControl|Sequence
        (:then_0
          (if (Variables|/Script/Engine.CharacterMovementComponent|GetbUseControllerDesiredRotation (Variables|/Script/Engine.Character|GetCharacterMovement (Variables|Default|GetRef_PlayerBP)))
            (switch string (Utilities|String|ToString(Text) (Class|KismetInputLibrary|KeyGetDisplayName (Variables|/Game/ThirdPerson/Blueprints/BP_ThirdPersonCharacter.BP_ThirdPersonCharacter_C|GetDirection%20Key (Variables|Default|GetRef_PlayerBP)) true))
              (:Z
                (Variables|Default|SetMovement%20Direction "NewEnumerator0"))
              (:Q
                (Variables|Default|SetMovement%20Direction "NewEnumerator1"))
              (:S
                (Variables|Default|SetMovement%20Direction "NewEnumerator2"))
              (:D
                (Variables|Default|SetMovement%20Direction "NewEnumerator3")))
            (else
              (Variables|Default|SetMovement%20Direction "NewEnumerator0"))))
        (:then_1
          (if (not (Variables|Default|GetIs%20Dodging))
            (Variables|Default|SetIs%20Dodging true)
            (Variables|Default|SetIsDodgingDone false)
            (Animation|Montage|PlayMontage (Variables|/Script/Engine.Character|GetMesh (Variables|Default|GetRef_PlayerBP)) (Utilities|Select :Index (Variables|Default|GetMovement%20Direction) :NewEnumerator0 "/Game/ARPG_Warrior/NewOscar/Dodge/Dodge_F_Montage.Dodge_F_Montage" :NewEnumerator1 "/Game/ARPG_Warrior/NewOscar/Dodge/Dodge_L_Montage.Dodge_L_Montage" :NewEnumerator2 "/Game/ARPG_Warrior/NewOscar/Dodge/Dodge_B_Montage.Dodge_B_Montage" :NewEnumerator3 "/Game/ARPG_Warrior/NewOscar/Dodge/Dodge_R_Montage.Dodge_R_Montage") 0.8
              (:then
                (Utilities|FlowControl|Sequence
                  (:then_0
                    ;;[0.2708 0.2708 0.2708 0.5] Pas fini besoin de trouver comment l'update pendant le roll
                    (Utilities|FlowControl|Delay 0.6)
                    (Variables|Default|SetIs%20Dodging false)
                    (Variables|/Script/Engine.CharacterMovementComponent|SetRotationRate (Variables|/Script/Engine.Character|GetCharacterMovement (Variables|Default|GetRef_PlayerBP)) "0.000000,850.000000,0.000000")
                    (Variables|/Game/Blueprints/BPC_Stats.BPC_Stats_C|SetStamina%20regain%20? _bpc_stats false)
                    (Default|IncreaseValue _bpc_stats "NewEnumerator2" -15.0))
                  (:then_1
                    (Utilities|FlowControl|Delay 0.55)
                    (Variables|Default|SetIsDodgingDone true)
                    (Variables|/Script/Engine.CharacterMovementComponent|SetRotationRate (Variables|/Script/Engine.Character|GetCharacterMovement (Variables|Default|GetRef_PlayerBP)) "0.000000,500.000000,0.000000")
                    (Variables|/Game/Blueprints/BPC_Stats.BPC_Stats_C|SetStamina%20regain%20? (Variables|/Game/ThirdPerson/Blueprints/BP_ThirdPersonCharacter.BP_ThirdPersonCharacter_C|GetBPC_Stats (Variables|Default|GetRef_PlayerBP)) true :!label _label))))
              (:OnCompleted
                (goto _label)))))))))

(event Input|EnhancedActionEvents|EnhancedInputActionIA_Lock
  (params (ActionValue :type Boolean) (ElapsedSeconds :type Float%20%28double-precision%29) (TriggeredSeconds :type Float%20%28double-precision%29) (InputAction :type Input%20Action%20Object%20Reference :default "/Game/Input/Actions/IA_Lock.IA_Lock"))
  (bind _returnvalue (Game|GetPlayerCameraManager 0))
  (bind _ref_playerbp (Variables|Default|GetRef_PlayerBP))
  (bind _ref_playerbp_2 (Variables|Default|GetRef_PlayerBP))
  (bind _transformcomponent (Variables|/Script/Engine.PlayerCameraManager|GetTransformComponent _returnvalue))
  (bind _charactermovement (Variables|/Script/Engine.Character|GetCharacterMovement _ref_playerbp))
  (bind _charactermovement_2 (Variables|/Script/Engine.Character|GetCharacterMovement _ref_playerbp_2))
  (bind _returnvalue_2 (Transformation|GetWorldLocation _transformcomponent))
  (bind _returnvalue_3 (+ (.z _returnvalue_2) 0.0))
  (bind _returnvalue_4 (Math|Vector|MakeVector (.x _returnvalue_2) (.y _returnvalue_2) _returnvalue_3))
  ;[0.2708 0.2708 0.2708 0.5] Target Lock
  (:Started
    (Variables|Default|GetTargetLockActor
      (:then
        (Variables|Default|SetTargetLockActor 0)
        (Variables|/Script/Engine.CharacterMovementComponent|SetbOrientRotationToMovement _charactermovement_2 true)
        (Variables|/Script/Engine.CharacterMovementComponent|SetbUseControllerDesiredRotation _charactermovement_2 false)
        (Actor|DestroyActor (Variables|Default|GetTargetLockWidget))
        (Variables|/Script/Engine.CharacterMovementComponent|SetRotationRate _charactermovement_2 "0.000000,500.000000,0.000000")
        (Utilities|IsValid (Variables|Default|GetTargetLockActor)
          (:Is%20Valid
            (Game|UnbindEventfromOnDestroyed (Variables|Default|GetTargetLockActor) (delegate Custom|DestroyWidget)))))
      (:else
        (bind (_outhit _returnvalue_5) (Collision|SphereTraceForObjects _returnvalue_4 (+ (* (Math|Vector|GetForwardVector (Transformation|GetWorldRotation _transformcomponent)) 1e+03) _returnvalue_4) 1.5e+02 (Utilities|Array|MakeArray "ObjectTypeQuery3") false 0 "ForDuration"))
        (if _returnvalue_5
          (Variables|Default|SetTargetLockActor (.HitActor (Collision|BreakHitResult _outhit)))
          (Variables|/Script/Engine.CharacterMovementComponent|SetbOrientRotationToMovement _charactermovement false)
          (Variables|/Script/Engine.CharacterMovementComponent|SetbUseControllerDesiredRotation _charactermovement true)
          (bind _returnvalue_6 (Game|SpawnActorfromClass "/Game/Blueprints/BP_TargetLockWidget.BP_TargetLockWidget_C" (Math|Transform|MakeTransform (Math|Vector|MakeVector (.x (.location (Transformation|GetActorTransform (Variables|Default|GetTargetLockActor)))) (.y (.location (Transformation|GetActorTransform (Variables|Default|GetTargetLockActor)))) (+ (.z (.location (Transformation|GetActorTransform (Variables|Default|GetTargetLockActor)))) 2e+01)) (.rotation (Transformation|GetActorTransform (Variables|Default|GetTargetLockActor))) (.scale (Transformation|GetActorTransform (Variables|Default|GetTargetLockActor)))) "AlwaysSpawn" "MultiplyWithRoot" 0 0))
          (bind _output_get (Variables|Default|SetTargetLockWidget _returnvalue_6))
          (Transformation|AttachActorToActor _output_get (Variables|Default|GetTargetLockActor) "None" "KeepWorld" "KeepRelative" "KeepRelative" true)
          (Variables|/Script/Engine.CharacterMovementComponent|SetRotationRate (Variables|/Script/Engine.Character|GetCharacterMovement (Variables|Default|GetRef_PlayerBP)) "0.000000,650.000000,0.000000")
          (Game|BindEventtoOnDestroyed (Variables|Default|GetTargetLockActor) (delegate Custom|DestroyWidget)))))))

(event EventTick
  (params (DeltaSeconds :type Float%20%28single-precision%29))
  (bind _ref_playerbp (Variables|Default|GetRef_PlayerBP))
  (bind _targetlockactor (Variables|Default|GetTargetLockActor))
  (bind _returnvalue (Transformation|GetActorLocation _targetlockactor))
  (bind _returnvalue_2 (Transformation|GetActorLocation _ref_playerbp))
  (bind _returnvalue_3 (Math|Rotator|FindLookatRotation _returnvalue_2 _returnvalue))
  ;[0.2708 0.2708 0.2708 0.5] Target Lock
  ;;[0.2708 0.2708 0.2708 0.5] Target Lock Update
  (Variables|Default|GetTargetLockActor
    (:then
      (Pawn|SetControlRotation (Pawn|GetController _ref_playerbp) (Math|Rotator|MakeRotator (.roll _returnvalue_3) (+ (.pitch _returnvalue_3) -2e+01) (.yaw _returnvalue_3))))
    (:else)))

(event EventBeginPlay
  ;[0.2708 0.2708 0.2708 0.5] Get Player Class
  (bind _asbp_third_person_character (Utilities|Casting|CastToBP_ThirdPersonCharacter (Components|GetOwner)))
  (Variables|Default|SetRef_PlayerBP _asbp_third_person_character))