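; Actor component that tracks player and enemy health and triggers the owner's death.
; IncreaseValue selects a stat, adds a signed value clamped between zero and its maximum, and prints the result.
; At zero it calls Die, which sends DieMessage to the owner.
; It also updates a progress bar supplied through SetHealthBarProgress, with both stats sharing that single widget reference.
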(event Custom|Die
  (Class|BPIDie|Die(Message) (Components|GetOwner)))

(event Custom|Set%20Health%20Bar%20Progress
  (params (HealthProgressBar :type Progress%20Bar%20Object%20Reference))
  (Variables|Default|SetHealth%20Progress%20Bar HealthProgressBar))

(fn IncreaseValue
  (params (Stat :type E_Stats%20Enum :default "NewEnumerator0") (Value :type Float%20%28double-precision%29))
  (switch Utilities|FlowControl|Switch|SwitchonE_Stats Stat
    (:NewEnumerator0
      ;[0.2708 0.2708 0.2708 0.5] Player Health Update
      (bind _output_get (Variables|Default|SetHealth (Math|Float|Clamp(Float) (+ (Variables|Default|GetHealth) Value) 0.0 (Variables|Default|GetMaxHealth))))
      (Development|PrintString (Utilities|String|ToString(Float) _output_get))
      (Utilities|FlowControl|Sequence
        (:then_0
          (if (<= (Variables|Default|GetHealth) 0.0)
            (CallFunction|Die)))
        (:then_1
          (bind _health_progress_bar (Variables|Default|GetHealth%20Progress%20Bar)
            (:then
              (Progress|SetPercent _health_progress_bar (/ (Variables|Default|GetHealth) (Variables|Default|GetMaxHealth))))
            (:else)))))
    (:NewEnumerator1
      ;[0.2708 0.2708 0.2708 0.5] Ennemy Health update
      (bind _output_get_2 (Variables|Default|SetEnnemyHealth (Math|Float|Clamp(Float) (+ (Variables|Default|GetEnnemyHealth) Value) 0.0 (Variables|Default|GetMaxEnnemyHealth))))
      (Development|PrintString (Utilities|String|ToString(Float) _output_get_2))
      (Utilities|FlowControl|Sequence
        (:then_0
          (if (<= (Variables|Default|GetEnnemyHealth) 0.0)
            (CallFunction|Die)))
        (:then_1
          (bind _health_progress_bar_2 (Variables|Default|GetHealth%20Progress%20Bar)
            (:then
              (Progress|SetPercent _health_progress_bar_2 (/ (Variables|Default|GetEnnemyHealth) (Variables|Default|GetMaxEnnemyHealth))))
            (:else)))))))